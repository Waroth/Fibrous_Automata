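; Interactive reaction-diffusion test actor that iterates a simulation material on render targets and displays it on a plane.
; Each tick alternates draws between two render targets, feeding the result back as the previous state.
; Held left mouse paints with a brush; keys 1 and 2 toggle stamping of the Hands texture and the scene capture's composite mode.
; Comma-separated Arduino serial readings drive the simulation's scale, diffusion and time parameters.
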(event Custom|Iterate
  (bind _rt (Variables|Default|GetRT))
  (bind _rt2 (Variables|Default|GetRT2))
  (Utilities|FlowControl|FlipFlop
    (:A
      (Rendering|DrawMaterialtoRenderTarget (Variables|Default|GetRT) (Variables|Default|GetMID_RD))
      (Rendering|Material|SetTextureParameterValue (Variables|Default|GetMID_RD) "Previous" _rt)
      (Rendering|Material|SetTextureParameterValue (Variables|Default|GetMID_Visualizer) "Texture" _rt))
    (:B
      (Rendering|DrawMaterialtoRenderTarget (Variables|Default|GetRT2) (Variables|Default|GetMID_RD))
      (Rendering|Material|SetTextureParameterValue (Variables|Default|GetMID_RD) "Previous" _rt2)
      (Rendering|Material|SetTextureParameterValue (Variables|Default|GetMID_Visualizer) "Texture" _rt2))))

(event Custom|DrawHands
  (bind _mid_hands (Variables|Default|GetMID_Hands))
  (if (Variables|Default|GetDrawMode)
    (Rendering|DrawMaterialtoRenderTarget (Variables|Default|GetRT) _mid_hands)
    (Rendering|DrawMaterialtoRenderTarget (Variables|Default|GetRT2) _mid_hands)
    (Rendering|Material|SetScalarParameterValue (Variables|Default|GetMID_RD) "DrawMode" 1.0 :!class /Script/Engine.MaterialInstanceDynamic)
    (Variables|/Script/Engine.SceneCaptureComponent2D|SetCompositeMode (Actor|GetComponentbyClass (Variables|Default|GetSceneCapture) "/Script/Engine.SceneCaptureComponent2D") "SCCM_Overwrite")
    (else
      (Rendering|Material|SetScalarParameterValue (Variables|Default|GetMID_RD) "DrawMode" 0.0 :!class /Script/Engine.MaterialInstanceDynamic)
      (Variables|/Script/Engine.SceneCaptureComponent2D|SetCompositeMode (Actor|GetComponentbyClass (Variables|Default|GetSceneCapture) "/Script/Engine.SceneCaptureComponent2D") "SCCM_Additive"))))

(event Custom|MouseTrace
  (bind _returnvalue (Game|GetPlayerController 0))
  (bind _mid_brush (Variables|Default|GetMID_Brush))
  (bind _hitresult (Game|Player|GetHitResultUnderCursorbyChannel _returnvalue "TraceTypeQuery1" false))
  (bind _impactpoint (Collision|BreakHitResult _hitresult))
  (bind (_x _y) (Math|Vector|BreakVector _impactpoint))
  (Utilities|FlowControl|Gate true
    (:Exit
      (Rendering|Material|SetVectorParameterValue (Variables|Default|GetMID_Brush) "Position" (Utilities|Struct|MakeLinearColor (+ (* (/ (+ (/ _x 21.0) 1.0) 2.0) 0.42) 0.29) (/ (+ (/ _y 5e+01) 1.0) 2.0) 0.0 0.0) :!class /Script/Engine.MaterialInstanceDynamic)
      (Rendering|DrawMaterialtoRenderTarget (Variables|Default|GetRT) _mid_brush)
      (Rendering|DrawMaterialtoRenderTarget (Variables|Default|GetRT2) _mid_brush))))

(event Custom|SetDynamicParameters
  (bind _dynamicvalues (Variables|Default|GetDynamicValues))
  (bind _mid_rd (Variables|Default|GetMID_RD))
  (Utilities|FlowControl|Sequence
    (:then_0
      (Rendering|Material|SetScalarParameterValue _mid_rd "Scale" (+ (- (Utilities|Array|Get(acopy) _dynamicvalues) 512.0) 3e+03) :!class /Script/Engine.MaterialInstanceDynamic))
    (:then_1
      (Rendering|Material|SetScalarParameterValue _mid_rd "dA" (* (/ (Utilities|Array|Get(acopy) _dynamicvalues 1) 1024.0) 2.0) :!class /Script/Engine.MaterialInstanceDynamic))
    (:then_2
      (Rendering|Material|SetScalarParameterValue _mid_rd "t" (/ (Utilities|Array|Get(acopy) _dynamicvalues 2) 1024.0) :!class /Script/Engine.MaterialInstanceDynamic))))

(event Custom|Arduino
  (bind _returnvalue (Class|ThreadBP|ReadSerial))
  (for (_array_element _array_index) (Utilities|String|ParseIntoArray _returnvalue ",")
    (Utilities|Array|SetArrayElem (Variables|Default|GetDynamicValues) _array_index (Math|Conversions|ToFloat(Integer) _array_element))))

(event EventBeginPlay
  (Variables|/Script/Engine.PlayerController|SetbShowMouseCursor (Game|GetPlayerController 0) false)
  (Rendering|ClearRenderTarget2D "/Game/Testing/Hands.Hands")
  (Rendering|Material|SetTextureParameterValue (Variables|Default|GetMID_Hands) "Texture" "/Game/Testing/Hands.Hands")
  (bind _outactors (Actor|GetAllActorsOfClass "/Script/Engine.SceneCapture2D"))
  (Variables|Default|SetSceneCapture (Utilities|Array|Get(acopy) _outactors))
  (Class|ThreadBP|OpenSerial 4 9600))

(event EventEndPlay
  (params (EndPlayReason :type EEndPlayReason%20Enum :default "Destroyed"))
  (Class|ThreadBP|CloseSerial))

(event EventTick
  (params (DeltaSeconds :type Float%20%28single-precision%29))
  (CallFunction|Iterate)
  (CallFunction|MouseTrace)
  (CallFunction|DrawHands)
  (CallFunction|Arduino)
  (CallFunction|SetDynamicParameters))

(event Input|KeyboardEvents|1
  (params (Key :type Key%20Structure :default "LeapLeftPinch"))
  (:Pressed
    (Variables|Default|SetDrawMode true)))

(event Input|KeyboardEvents|2
  (params (Key :type Key%20Structure :default "LeapLeftPinch"))
  (:Pressed
    (Variables|Default|SetDrawMode false)))

(event Input|MouseEvents|LeftMouseButton
  (params (Key :type Key%20Structure :default "AnyKey"))
  (bind _returnvalue (Game|GetPlayerController 0))
  (bind _mid_brush (Variables|Default|GetMID_Brush))
  (bind _hitresult (Game|Player|GetHitResultUnderCursorbyChannel _returnvalue "TraceTypeQuery1" false))
  (bind _impactpoint (Collision|BreakHitResult _hitresult))
  (bind (_x _y) (Math|Vector|BreakVector _impactpoint))
  (:Pressed
    (Utilities|FlowControl|Gate true) ; enters at Open
  )
  (:Released
    (Utilities|FlowControl|Gate true) ; enters at Close
  ))

(fn ConstructionScript
  (Utilities|FlowControl|Sequence
    (:then_0
      (bind _returnvalue (Rendering|Material|CreateDynamicMaterialInstance "/Game/Testing/Reaction_Diffusion.Reaction_Diffusion" :!class /Script/Engine.KismetMaterialLibrary))
      (bind _output_get (Variables|Default|SetMID_RD _returnvalue))
      (bind _returnvalue_2 (Rendering|Material|CreateDynamicMaterialInstance (Variables|Default|GetPlane) 0 "/Game/Testing/M_MultiVisualizer.M_MultiVisualizer" :!class /Script/Engine.PrimitiveComponent))
      (Variables|Default|SetMID_Visualizer _returnvalue_2)
      (Rendering|Material|SetMaterial (Variables|Default|GetPlane) 0 _output_get))
    (:then_1
      (bind _returnvalue_3 (Rendering|Material|CreateDynamicMaterialInstance "/Game/Testing/M_Brush.M_Brush" :!class /Script/Engine.KismetMaterialLibrary))
      (Variables|Default|SetMID_Brush _returnvalue_3)
      (bind _returnvalue_4 (Rendering|Material|CreateDynamicMaterialInstance "/Game/Testing/M_HandBrush.M_HandBrush" :!class /Script/Engine.KismetMaterialLibrary))
      (Variables|Default|SetMID_Hands _returnvalue_4))))